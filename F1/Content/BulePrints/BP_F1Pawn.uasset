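; BP_F1Pawn is a player-controlled pawn that moves and turns through Enhanced Input.
; BeginPlay adds the IMC_Defalult mapping context to the owning player controller.
; IA_Move feeds world-space forward and right vectors, scaled by input, into local offsets without sweep, so direction compounds with actor rotation.
; IA_Turn adds local yaw directly from input; neither action scales by delta time.
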(event Input|EnhancedActionEvents|EnhancedInputActionIA_Move
  (params (ActionValue :type Vector%202D%20Structure) (ElapsedSeconds :type Float%20%28double-precision%29) (TriggeredSeconds :type Float%20%28double-precision%29) (InputAction :type Input%20Action%20Object%20Reference :default "/Game/Input/Actons/IA_Move.IA_Move"))
  (:Triggered
    (Transformation|AddActorLocalOffset (* (Transformation|GetActorForwardVector) (.x ActionValue)) false false)
    (Transformation|AddActorLocalOffset (* (Transformation|GetActorRightVector) (.y ActionValue)) false false)))

(event Input|EnhancedActionEvents|EnhancedInputActionIA_Turn
  (params (ActionValue :type Vector%202D%20Structure) (ElapsedSeconds :type Float%20%28double-precision%29) (TriggeredSeconds :type Float%20%28double-precision%29) (InputAction :type Input%20Action%20Object%20Reference :default "/Game/Input/Actons/IA_Turn.IA_Turn"))
  (:Triggered
    (Transformation|AddActorLocalRotation (Math|Rotator|MakeRotator 0.0 0.0 (.x ActionValue)) false false)))

(event EventBeginPlay
  (bind _asplayer_controller (Utilities|Casting|CastToPlayerController (Pawn|GetController)))
  (Input|AddMappingContext (PlayerController|LocalPlayerSubsystems|GetEnhancedInputLocalPlayerSubsystem _asplayer_controller) "/Game/Input/IMC_Defalult.IMC_Defalult" 0 "(bIgnoreAllPressedKeysUntilRelease=True,bForceImmediately=False,bNotifyUserSettings=False)"))

(event Collision|EventActorBeginOverlap
  (params (OtherActor :type Actor%20Object%20Reference)))

(event EventTick
  (params (DeltaSeconds :type Float%20%28single-precision%29)))

(fn ConstructionScript)